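; Sanity system controller that raises or drains the player's SanityLevel every tick, clamped between 0 and 100.
; Sanity rises while SanityZoneCheck is true or the first-person character's flashlight toggle is on, and falls otherwise.
; The increase and decrease speeds apply per frame, as the stored DeltaTime is unused in the calculation.
; The current level is printed on screen as debug output.
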(event `self.ReceiveBeginPlay`)

(event `self.ReceiveTick`
  (params (DeltaSeconds :type "Float (single-precision)"))
  (bind _sanitylevel (`self.SanityLevel`))
  (bind _sanitylevel_2 (`self.SanityLevel`))
  (set `self.DeltaTime` DeltaSeconds)
  (bind _asbp_first_person_character (cast `/Game/FirstPerson/Blueprints/BP_FirstPersonCharacter` (`GameplayStatics.GetPlayerCharacter` 0)))
  (if (or (`self.SanityZoneCheck`) (`/Game/FirstPerson/Blueprints/BP_FirstPersonCharacter.Flashlight Toggle` _asbp_first_person_character))
    (bind _output_get (set `self.SanityLevel` (+ (`self.SanityIncreaseSpeed`) _sanitylevel_2)))
    (set `self.SanityLevel` (`KismetMathLibrary.FClamp` _output_get 0.0 100.0))
    (`KismetSystemLibrary.PrintString` (`KismetStringLibrary.BuildString_Double` "" "SanityLevel: " _sanitylevel) true false (struct :`G` 0.66 :`B` 1.0 :`A` 1.0) 0.5)
    (else
      (bind _output_get_2 (set `self.SanityLevel` (- _sanitylevel_2 (`self.SanityDecreaseSpeed`))))
      (set `self.SanityLevel` (`KismetMathLibrary.FClamp` _output_get_2 0.0 100.0))
      (`KismetSystemLibrary.PrintString` (`KismetStringLibrary.BuildString_Double` "" "SanityLevel: " _sanitylevel) true false (struct :`G` 0.66 :`B` 1.0 :`A` 1.0) 0.5))))